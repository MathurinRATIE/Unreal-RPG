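; Quest manager that tracks the player's claimed, active and finished RPG quests, their stage progression and their rewards.
; Claiming builds a mutable, ID-keyed progress copy (ManipulatedQuests) of the data asset's stages and objectives.
; Collect, kill, location and speak checks complete current-stage objectives.
; End-stage-checker objectives trigger stage completion, which advances or finishes the quest and grants rewards, adding items only when inventory space allows.
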(event `self.ReceiveBeginPlay`
  (bind _asbp_player (cast `/Game/RPG/Player/BP_Player` (`GameplayStatics.GetPlayerCharacter` 0)))
  (set `self.BP Player` _asbp_player))

(fn `CheckCollectObjectives`
  (locals (CanBeCompleted :type Boolean) (CurrentQuest :type "/Game/RPG/Blueprints/QuestsSystem/QuestsDatas/PDA_Quest Object Reference") (CurrentObjectiveDatas :type "/Game/RPG/Blueprints/QuestsSystem/QuestsDatas/PDA_Objective Object Reference") (CurrentQuestIndex :type Integer) (CurrentObjective :type "/Game/RPG/Blueprints/QuestsSystem/QuestsDatas/S_ManipulatedObjective Structure"))
  (bind _output_id (break `/Game/RPG/Blueprints/QuestsSystem/QuestsDatas/S_ManipulatedQuest` (`|GetArrayItem` (`self.ManipulatedQuests`) (`local.CurrentQuestIndex`))))
  (bind (_output_id_2 _output_stages _output_currentstage) (break `/Game/RPG/Blueprints/QuestsSystem/QuestsDatas/S_ManipulatedQuest` (`|GetArrayItem` (`self.ManipulatedQuests`) (`local.CurrentQuestIndex`))))
  (bind (_questdatas_id _questdatas_name _questdatas_description _questdatas_stages) (break `/Game/RPG/Blueprints/QuestsSystem/QuestsDatas/S_Quest` (`/Game/RPG/Blueprints/QuestsSystem/QuestsDatas/PDA_Quest.QuestDatas` (`local.CurrentQuest`))))
  (bind _output_id_3 (break `/Game/RPG/Blueprints/QuestsSystem/QuestsDatas/S_ManipulatedStage` (`|GetArrayItem` _output_stages _output_currentstage)))
  (for _array_element (`self.StartedQuests`)
    (bind _output_get (set `local.CurrentQuest` _array_element))
    (bind _questdatas_id_2 (break `/Game/RPG/Blueprints/QuestsSystem/QuestsDatas/S_Quest` (`/Game/RPG/Blueprints/QuestsSystem/QuestsDatas/PDA_Quest.QuestDatas` _output_get)))
    (bind _index (`self.GetManipulatedQuestIndexByQuestID` _questdatas_id_2))
    (bind _output_get_2 (set `local.CurrentQuestIndex` _index))
    (bind (_output_id_4 _output_stages_2 _output_currentstage_2) (break `/Game/RPG/Blueprints/QuestsSystem/QuestsDatas/S_ManipulatedQuest` (`|GetArrayItem` (`self.ManipulatedQuests`) _output_get_2)))
    (bind (_stagedatas_id _stagedatas_name _stagedatas_description _stagedatas_objectives) (break `/Game/RPG/Blueprints/QuestsSystem/QuestsDatas/S_Stage` (`/Game/RPG/Blueprints/QuestsSystem/QuestsDatas/PDA_Stage.StageDatas` (`|GetArrayItem` _questdatas_stages _output_currentstage_2))))
    (for _array_element_2 _stagedatas_objectives
      (bind _output_get_3 (set `local.CurrentObjectiveDatas` _array_element_2))
      (bind (_objectivedatas_id _objectivedatas_name _objectivedatas_description _objectivedatas_type) (break `/Game/RPG/Blueprints/QuestsSystem/QuestsDatas/S_Objective` (`/Game/RPG/Blueprints/QuestsSystem/QuestsDatas/PDA_Objective.ObjectiveDatas` _output_get_3)))
      (bind _objective (`self.GetManipulatedObjectiveByUpIDs` _output_id_2 _output_id_3 _objectivedatas_id))
      (bind _output_get_4 (set `local.CurrentObjective` _objective))
      (bind _aspda_objective_collect (cast `/Game/RPG/Blueprints/QuestsSystem/QuestsDatas/PDA_ObjectiveCollect` (`local.CurrentObjectiveDatas`)))
      (if (and (`|EnumEquality` _objectivedatas_type "NewEnumerator0") (or (`/Game/RPG/Blueprints/QuestsSystem/QuestsDatas/PDA_ObjectiveCollect.Consume` _aspda_objective_collect) (not (`.IsCompleted_4_0007CAF040ABB7D21F1D118472BE4227` (break `/Game/RPG/Blueprints/QuestsSystem/QuestsDatas/S_ManipulatedObjective` _output_get_4)))))
        (set `local.CanBeCompleted` true)
        (for _array_element_3 (`/Game/RPG/Blueprints/QuestsSystem/QuestsDatas/PDA_ObjectiveCollect.Items` _aspda_objective_collect)
          (bind _inventorycount (`/Game/RPG/Player/Components/BPC_Inventory.GetItemAmount` (`/Game/RPG/Player/BP_Player.PBC_Inventory` (`self.BP Player`)) (break `/Game/RPG/Blueprints/Item/S_ItemSlot` _array_element_3)))
          (if (not (>= _inventorycount (`.Amount_7_E08AD9B3421E831788A24AA7FF7CCAA7` (break `/Game/RPG/Blueprints/Item/S_ItemSlot` _array_element_3))))
            (set `local.CanBeCompleted` false)
            (break)))
        (if (`local.CanBeCompleted`)
          (`self.CompleteObjective` (`local.CurrentObjectiveDatas`) (`local.CurrentQuest`))
          (else
            (`self.Set Objective Completion` (`local.CurrentObjectiveDatas`) _output_id false)))))))

(fn `CheckInteractObjectives`
  (params (PNJ :type "/Game/RPG/Blueprints/PNJs/BP_PNJ Object Reference"))
  (locals (`PNJ ID` :type Integer :default 0) (CurrentQuest :type "/Game/RPG/Blueprints/QuestsSystem/QuestsDatas/PDA_Quest Object Reference") (CurrentObjectiveDatas :type "/Game/RPG/Blueprints/QuestsSystem/QuestsDatas/PDA_Objective Object Reference") (CurrentQuestIndex :type Integer) (CurrentObjective :type "/Game/RPG/Blueprints/QuestsSystem/QuestsDatas/S_ManipulatedObjective Structure"))
  (bind (_output_id _output_stages _output_currentstage) (break `/Game/RPG/Blueprints/QuestsSystem/QuestsDatas/S_ManipulatedQuest` (`|GetArrayItem` (`self.ManipulatedQuests`) (`local.CurrentQuestIndex`))))
  (bind (_questdatas_id _questdatas_name _questdatas_description _questdatas_stages) (break `/Game/RPG/Blueprints/QuestsSystem/QuestsDatas/S_Quest` (`/Game/RPG/Blueprints/QuestsSystem/QuestsDatas/PDA_Quest.QuestDatas` (`local.CurrentQuest`))))
  (bind _output_id_2 (break `/Game/RPG/Blueprints/QuestsSystem/QuestsDatas/S_ManipulatedStage` (`|GetArrayItem` _output_stages _output_currentstage)))
  (set `local.PNJ ID` (`/Game/RPG/Blueprints/PNJs/BP_PNJ.ID` PNJ))
  (for _array_element (`self.StartedQuests`)
    (bind _output_get (set `local.CurrentQuest` _array_element))
    (bind _questdatas_id_2 (break `/Game/RPG/Blueprints/QuestsSystem/QuestsDatas/S_Quest` (`/Game/RPG/Blueprints/QuestsSystem/QuestsDatas/PDA_Quest.QuestDatas` _output_get)))
    (bind _index (`self.GetManipulatedQuestIndexByQuestID` _questdatas_id_2))
    (bind _output_get_2 (set `local.CurrentQuestIndex` _index))
    (bind (_output_id_3 _output_stages_2 _output_currentstage_2) (break `/Game/RPG/Blueprints/QuestsSystem/QuestsDatas/S_ManipulatedQuest` (`|GetArrayItem` (`self.ManipulatedQuests`) _output_get_2)))
    (bind (_stagedatas_id _stagedatas_name _stagedatas_description _stagedatas_objectives) (break `/Game/RPG/Blueprints/QuestsSystem/QuestsDatas/S_Stage` (`/Game/RPG/Blueprints/QuestsSystem/QuestsDatas/PDA_Stage.StageDatas` (`|GetArrayItem` _questdatas_stages _output_currentstage_2))))
    (for _array_element_2 _stagedatas_objectives
      (bind _output_get_3 (set `local.CurrentObjectiveDatas` _array_element_2))
      (bind (_objectivedatas_id _objectivedatas_name _objectivedatas_description _objectivedatas_type) (break `/Game/RPG/Blueprints/QuestsSystem/QuestsDatas/S_Objective` (`/Game/RPG/Blueprints/QuestsSystem/QuestsDatas/PDA_Objective.ObjectiveDatas` _output_get_3)))
      (bind _objective (`self.GetManipulatedObjectiveByUpIDs` _output_id _output_id_2 _objectivedatas_id))
      (bind _output_get_4 (set `local.CurrentObjective` _objective))
      (if (and (not (`.IsCompleted_4_0007CAF040ABB7D21F1D118472BE4227` (break `/Game/RPG/Blueprints/QuestsSystem/QuestsDatas/S_ManipulatedObjective` _output_get_4))) (`|EnumEquality` _objectivedatas_type "NewEnumerator3"))
        (bind _aspda_objective_speak (cast `/Game/RPG/Blueprints/QuestsSystem/QuestsDatas/PDA_ObjectiveSpeak` (`local.CurrentObjectiveDatas`)))
        (if (== (`/Game/RPG/Blueprints/QuestsSystem/QuestsDatas/PDA_ObjectiveSpeak.PNJ_ID` _aspda_objective_speak) (`local.PNJ ID`))
          (`self.CompleteObjective` (`local.CurrentObjectiveDatas`) (`local.CurrentQuest`)))))))

(fn `CheckKillObjectives`
  (params (EnemyKilled :type "/Game/RPG/Blueprints/Ennemies/BP_Enemy Object Reference"))
  (locals (EnemyKilledID :type Integer) (CurrentQuest :type "/Game/RPG/Blueprints/QuestsSystem/QuestsDatas/PDA_Quest Object Reference") (CurrentObjectiveDatas :type "/Game/RPG/Blueprints/QuestsSystem/QuestsDatas/PDA_Objective Object Reference") (CurrentQuestIndex :type Integer) (CurrentObjective :type "/Game/RPG/Blueprints/QuestsSystem/QuestsDatas/S_ManipulatedObjective Structure"))
  (bind (_output_id _output_stages _output_currentstage) (break `/Game/RPG/Blueprints/QuestsSystem/QuestsDatas/S_ManipulatedQuest` (`|GetArrayItem` (`self.ManipulatedQuests`) (`local.CurrentQuestIndex`))))
  (bind (_questdatas_id _questdatas_name _questdatas_description _questdatas_stages) (break `/Game/RPG/Blueprints/QuestsSystem/QuestsDatas/S_Quest` (`/Game/RPG/Blueprints/QuestsSystem/QuestsDatas/PDA_Quest.QuestDatas` (`local.CurrentQuest`))))
  (bind _output_id_2 (break `/Game/RPG/Blueprints/QuestsSystem/QuestsDatas/S_ManipulatedStage` (`|GetArrayItem` _output_stages _output_currentstage)))
  (set `local.EnemyKilledID` (`/Game/RPG/Blueprints/Ennemies/BP_Enemy.ID` EnemyKilled))
  (for _array_element (`self.StartedQuests`)
    (bind _output_get (set `local.CurrentQuest` _array_element))
    (bind _questdatas_id_2 (break `/Game/RPG/Blueprints/QuestsSystem/QuestsDatas/S_Quest` (`/Game/RPG/Blueprints/QuestsSystem/QuestsDatas/PDA_Quest.QuestDatas` _output_get)))
    (bind _index (`self.GetManipulatedQuestIndexByQuestID` _questdatas_id_2))
    (bind _output_get_2 (set `local.CurrentQuestIndex` _index))
    (bind (_output_id_3 _output_stages_2 _output_currentstage_2) (break `/Game/RPG/Blueprints/QuestsSystem/QuestsDatas/S_ManipulatedQuest` (`|GetArrayItem` (`self.ManipulatedQuests`) _output_get_2)))
    (bind (_stagedatas_id _stagedatas_name _stagedatas_description _stagedatas_objectives) (break `/Game/RPG/Blueprints/QuestsSystem/QuestsDatas/S_Stage` (`/Game/RPG/Blueprints/QuestsSystem/QuestsDatas/PDA_Stage.StageDatas` (`|GetArrayItem` _questdatas_stages _output_currentstage_2))))
    (for _array_element_2 _stagedatas_objectives
      (bind _output_get_3 (set `local.CurrentObjectiveDatas` _array_element_2))
      (bind (_objectivedatas_id _objectivedatas_name _objectivedatas_description _objectivedatas_type) (break `/Game/RPG/Blueprints/QuestsSystem/QuestsDatas/S_Objective` (`/Game/RPG/Blueprints/QuestsSystem/QuestsDatas/PDA_Objective.ObjectiveDatas` _output_get_3)))
      (bind _objective (`self.GetManipulatedObjectiveByUpIDs` _output_id _output_id_2 _objectivedatas_id))
      (bind _output_get_4 (set `local.CurrentObjective` _objective))
      (if (and (not (`.IsCompleted_4_0007CAF040ABB7D21F1D118472BE4227` (break `/Game/RPG/Blueprints/QuestsSystem/QuestsDatas/S_ManipulatedObjective` _output_get_4))) (`|EnumEquality` _objectivedatas_type "NewEnumerator1"))
        (bind _aspda_objective_kill (cast `/Game/RPG/Blueprints/QuestsSystem/QuestsDatas/PDA_ObjectiveKill` (`local.CurrentObjectiveDatas`)))
        (if (== (`/Game/RPG/Blueprints/QuestsSystem/QuestsDatas/PDA_ObjectiveKill.EnemyID` _aspda_objective_kill) (`local.EnemyKilledID`))
          (`self.CompleteObjective` (`local.CurrentObjectiveDatas`) (`local.CurrentQuest`)))))))

(fn `CheckLocationObjectives`
  (params (Waypoint :type "/Game/RPG/Blueprints/QuestsSystem/BP_Waypoint Object Reference"))
  (locals (AcceptenceDistance :type "Float (double-precision)" :default 50.0) (CurrentQuest :type "/Game/RPG/Blueprints/QuestsSystem/QuestsDatas/PDA_Quest Object Reference") (CurrentObjectiveDatas :type "/Game/RPG/Blueprints/QuestsSystem/QuestsDatas/PDA_Objective Object Reference") (CurrentWaypoint :type "/Game/RPG/Blueprints/QuestsSystem/BP_Waypoint Object Reference") (CurrentQuestIndex :type Integer) (CurrentObjective :type "/Game/RPG/Blueprints/QuestsSystem/QuestsDatas/S_ManipulatedObjective Structure"))
  (bind (_output_id _output_stages _output_currentstage) (break `/Game/RPG/Blueprints/QuestsSystem/QuestsDatas/S_ManipulatedQuest` (`|GetArrayItem` (`self.ManipulatedQuests`) (`local.CurrentQuestIndex`))))
  (bind (_questdatas_id _questdatas_name _questdatas_description _questdatas_stages) (break `/Game/RPG/Blueprints/QuestsSystem/QuestsDatas/S_Quest` (`/Game/RPG/Blueprints/QuestsSystem/QuestsDatas/PDA_Quest.QuestDatas` (`local.CurrentQuest`))))
  (bind _output_id_2 (break `/Game/RPG/Blueprints/QuestsSystem/QuestsDatas/S_ManipulatedStage` (`|GetArrayItem` _output_stages _output_currentstage)))
  (set `local.CurrentWaypoint` Waypoint)
  (for _array_element (`self.StartedQuests`)
    (bind _output_get (set `local.CurrentQuest` _array_element))
    (bind _questdatas_id_2 (break `/Game/RPG/Blueprints/QuestsSystem/QuestsDatas/S_Quest` (`/Game/RPG/Blueprints/QuestsSystem/QuestsDatas/PDA_Quest.QuestDatas` _output_get)))
    (bind _index (`self.GetManipulatedQuestIndexByQuestID` _questdatas_id_2))
    (bind _output_get_2 (set `local.CurrentQuestIndex` _index))
    (bind (_output_id_3 _output_stages_2 _output_currentstage_2) (break `/Game/RPG/Blueprints/QuestsSystem/QuestsDatas/S_ManipulatedQuest` (`|GetArrayItem` (`self.ManipulatedQuests`) _output_get_2)))
    (bind (_stagedatas_id _stagedatas_name _stagedatas_description _stagedatas_objectives) (break `/Game/RPG/Blueprints/QuestsSystem/QuestsDatas/S_Stage` (`/Game/RPG/Blueprints/QuestsSystem/QuestsDatas/PDA_Stage.StageDatas` (`|GetArrayItem` _questdatas_stages _output_currentstage_2))))
    (for _array_element_2 _stagedatas_objectives
      (bind _output_get_3 (set `local.CurrentObjectiveDatas` _array_element_2))
      (bind (_objectivedatas_id _objectivedatas_name _objectivedatas_description _objectivedatas_type) (break `/Game/RPG/Blueprints/QuestsSystem/QuestsDatas/S_Objective` (`/Game/RPG/Blueprints/QuestsSystem/QuestsDatas/PDA_Objective.ObjectiveDatas` _output_get_3)))
      (bind _objective (`self.GetManipulatedObjectiveByUpIDs` _output_id _output_id_2 _objectivedatas_id))
      (bind _output_get_4 (set `local.CurrentObjective` _objective))
      (if (and (not (`.IsCompleted_4_0007CAF040ABB7D21F1D118472BE4227` (break `/Game/RPG/Blueprints/QuestsSystem/QuestsDatas/S_ManipulatedObjective` _output_get_4))) (`|EnumEquality` _objectivedatas_type "NewEnumerator2"))
        (bind _aspda_objective_location (cast `/Game/RPG/Blueprints/QuestsSystem/QuestsDatas/PDA_ObjectiveLocation` (`local.CurrentObjectiveDatas`)))
        (if (== (`/Game/RPG/Blueprints/QuestsSystem/QuestsDatas/PDA_ObjectiveLocation.WaypointID` _aspda_objective_location) (`/Game/RPG/Blueprints/QuestsSystem/BP_Waypoint.ID` (`local.CurrentWaypoint`)))
          (`self.CompleteObjective` (`local.CurrentObjectiveDatas`) (`local.CurrentQuest`)))))))

(fn `CheckStageFinished`
  (params (QuestDatas :type "/Game/RPG/Blueprints/QuestsSystem/QuestsDatas/PDA_Quest Object Reference"))
  (returns (AllObjectivesCompleted :type Boolean))
  (locals (AllCompleted :type Boolean) (QuestID :type Integer))
  (bind (_questdatas_id _questdatas_name _questdatas_description _questdatas_stages) (break `/Game/RPG/Blueprints/QuestsSystem/QuestsDatas/S_Quest` (`/Game/RPG/Blueprints/QuestsSystem/QuestsDatas/PDA_Quest.QuestDatas` QuestDatas)))
  (bind _quest (`self.GetManipulatedQuestByQuestID` _questdatas_id))
  (set `local.QuestID` (break `/Game/RPG/Blueprints/QuestsSystem/QuestsDatas/S_ManipulatedQuest` _quest))
  (set `local.AllCompleted` true)
  (bind (_stagedatas_id _stagedatas_name _stagedatas_description _stagedatas_objectives) (break `/Game/RPG/Blueprints/QuestsSystem/QuestsDatas/S_Stage` (`/Game/RPG/Blueprints/QuestsSystem/QuestsDatas/PDA_Stage.StageDatas` (`|GetArrayItem` _questdatas_stages (`.CurrentStage_10_E1FC846D4FAE690A0C9C04AF3D12109D` (break `/Game/RPG/Blueprints/QuestsSystem/QuestsDatas/S_ManipulatedQuest` _quest))))))
  (for _array_element _stagedatas_objectives
    (bind _quest_2 (`self.GetManipulatedQuestByQuestID` (`local.QuestID`)))
    (bind _output_id (break `/Game/RPG/Blueprints/QuestsSystem/QuestsDatas/S_ManipulatedStage` (`|GetArrayItem` (`.Stages_12_59DF7918458BD96E23CA02A4A01EEF48` (break `/Game/RPG/Blueprints/QuestsSystem/QuestsDatas/S_ManipulatedQuest` _quest_2)) (`.CurrentStage_10_E1FC846D4FAE690A0C9C04AF3D12109D` (break `/Game/RPG/Blueprints/QuestsSystem/QuestsDatas/S_ManipulatedQuest` _quest_2)))))
    (bind (_objectivedatas_id _objectivedatas_name _objectivedatas_description _objectivedatas_type _objectivedatas_approximatelocation _objectivedatas_optional _objectivedatas_optionalexperiencereward _objectivedatas_optionalmoneyreward _objectivedatas_optionalitemsreward _objectivedatas_endstagechecker) (break `/Game/RPG/Blueprints/QuestsSystem/QuestsDatas/S_Objective` (`/Game/RPG/Blueprints/QuestsSystem/QuestsDatas/PDA_Objective.ObjectiveDatas` _array_element)))
    (bind _objective (`self.GetManipulatedObjectiveByUpIDs` (break `/Game/RPG/Blueprints/QuestsSystem/QuestsDatas/S_ManipulatedQuest` _quest_2) _output_id _objectivedatas_id))
    (if (not (or (`.IsCompleted_4_0007CAF040ABB7D21F1D118472BE4227` (break `/Game/RPG/Blueprints/QuestsSystem/QuestsDatas/S_ManipulatedObjective` _objective)) _objectivedatas_optional _objectivedatas_endstagechecker))
      (set `local.AllCompleted` false)
      (break)))
  (return (`local.AllCompleted`)))

(fn `ClaimQuest`
  (params (QuestDatas :type "/Game/RPG/Blueprints/QuestsSystem/QuestsDatas/PDA_Quest Object Reference"))
  (`KismetArrayLibrary.Array_AddUnique` (`self.StartedQuests`) QuestDatas)
  (`KismetArrayLibrary.Array_RemoveItem` (`self.InactiveQuests`) QuestDatas)
  (bind _manipulatedquest (`self.CreateManipulatedQuest` QuestDatas))
  (`KismetArrayLibrary.Array_AddUnique` (`self.ManipulatedQuests`) _manipulatedquest)
  (`/Engine/EditorBlueprintResources/StandardMacros.IsValid` (`self.ActiveQuest`)
    (:`Is Not Valid`
      (`self.SetQuestActive` QuestDatas))))

(fn `ClaimQuestRawards`
  (params (StagesDatas :type "Array of /Game/RPG/Blueprints/QuestsSystem/QuestsDatas/PDA_Stage Object Reference") (CurrentStage :type Integer) (QuestID :type Integer) (StageCompletion :type Boolean))
  (for _array_element StagesDatas
    (bind _stagedatas_id (break `/Game/RPG/Blueprints/QuestsSystem/QuestsDatas/S_Stage` (`/Game/RPG/Blueprints/QuestsSystem/QuestsDatas/PDA_Stage.StageDatas` _array_element)))
    (bind (_stage _index) (`self.GetManipulatedStageByUpIDs` QuestID _stagedatas_id))
    (if (and (not (`.ItemRewardClaimed_9_33EA2BE74F3E9AF84DEA458FB561CCFC` (break `/Game/RPG/Blueprints/QuestsSystem/QuestsDatas/S_ManipulatedStage` _stage))) (<= _index CurrentStage))
      (if (and (== _index (- CurrentStage 1)) StageCompletion)
        (`self.ClaimStageRewards` _array_element QuestID)
        (else
          (`self.ClaimStageItemRewards` _array_element QuestID))))))

(fn `ClaimStageItemRewards`
  (params (StageDatas :type "/Game/RPG/Blueprints/QuestsSystem/QuestsDatas/PDA_Stage Object Reference") (QuestID :type Integer))
  (locals (ItemsToAdd :type "Array of /Game/RPG/Blueprints/Item/S_ItemSlot Structure"))
  (bind (_stagedatas_id _stagedatas_name _stagedatas_description _stagedatas_objectives _stagedatas_experiencereward _stagedatas_moneyreward _stagedatas_itemsreward) (break `/Game/RPG/Blueprints/QuestsSystem/QuestsDatas/S_Stage` (`/Game/RPG/Blueprints/QuestsSystem/QuestsDatas/PDA_Stage.StageDatas` StageDatas)))
  (set `local.ItemsToAdd` _stagedatas_itemsreward)
  (for _array_element _stagedatas_objectives
    (bind (_objectivedatas_id _objectivedatas_name _objectivedatas_description _objectivedatas_type _objectivedatas_approximatelocation _objectivedatas_optional _objectivedatas_optionalexperiencereward _objectivedatas_optionalmoneyreward _objectivedatas_optionalitemsreward) (break `/Game/RPG/Blueprints/QuestsSystem/QuestsDatas/S_Objective` (`/Game/RPG/Blueprints/QuestsSystem/QuestsDatas/PDA_Objective.ObjectiveDatas` _array_element)))
    (if _objectivedatas_optional
      (for _array_element_2 _objectivedatas_optionalitemsreward
        (`KismetArrayLibrary.Array_Add` (`local.ItemsToAdd`) _array_element_2))))
  (bind _canaddall (`/Game/RPG/Player/Components/BPC_Inventory.CanAdd` (`/Game/RPG/Player/BP_Player.PBC_Inventory` (`self.BP Player`)) (`local.ItemsToAdd`)))
  (if _canaddall
    (`self.SetStageRewardsClaimed` StageDatas QuestID)
    (for _array_element_3 (`local.ItemsToAdd`)
      (`/Game/RPG/Player/Components/BPC_Inventory.AddItem` (`/Game/RPG/Player/BP_Player.PBC_Inventory` (`self.BP Player`)) (break `/Game/RPG/Blueprints/Item/S_ItemSlot` _array_element_3) (`.Amount_7_E08AD9B3421E831788A24AA7FF7CCAA7` (break `/Game/RPG/Blueprints/Item/S_ItemSlot` _array_element_3))))))

(fn `ClaimStageRewards`
  (params (StageDatas :type "/Game/RPG/Blueprints/QuestsSystem/QuestsDatas/PDA_Stage Object Reference") (QuestID :type Integer))
  (locals (ItemsToAdd :type "Array of /Game/RPG/Blueprints/Item/S_ItemSlot Structure"))
  (bind (_stagedatas_id _stagedatas_name _stagedatas_description _stagedatas_objectives _stagedatas_experiencereward _stagedatas_moneyreward) (break `/Game/RPG/Blueprints/QuestsSystem/QuestsDatas/S_Stage` (`/Game/RPG/Blueprints/QuestsSystem/QuestsDatas/PDA_Stage.StageDatas` StageDatas)))
  (`/Game/RPG/Player/BP_Player.AddExp` (`self.BP Player`) _stagedatas_experiencereward)
  (`/Game/RPG/Player/BP_Player.AddMoney` (`self.BP Player`) _stagedatas_moneyreward)
  (for _array_element _stagedatas_objectives
    (bind (_objectivedatas_id _objectivedatas_name _objectivedatas_description _objectivedatas_type _objectivedatas_approximatelocation _objectivedatas_optional _objectivedatas_optionalexperiencereward _objectivedatas_optionalmoneyreward) (break `/Game/RPG/Blueprints/QuestsSystem/QuestsDatas/S_Objective` (`/Game/RPG/Blueprints/QuestsSystem/QuestsDatas/PDA_Objective.ObjectiveDatas` _array_element)))
    (if _objectivedatas_optional
      (`/Game/RPG/Player/BP_Player.AddExp` (`self.BP Player`) _objectivedatas_optionalexperiencereward)
      (`/Game/RPG/Player/BP_Player.AddMoney` (`self.BP Player`) _objectivedatas_optionalmoneyreward)))
  (`self.ClaimStageItemRewards` StageDatas QuestID))

(fn `CompleteObjective`
  (params (ObjectiveDatas :type "/Game/RPG/Blueprints/QuestsSystem/QuestsDatas/PDA_Objective Object Reference") (QuestDatas :type "/Game/RPG/Blueprints/QuestsSystem/QuestsDatas/PDA_Quest Object Reference"))
  (bind (_questdatas_id _questdatas_name _questdatas_description _questdatas_stages) (break `/Game/RPG/Blueprints/QuestsSystem/QuestsDatas/S_Quest` (`/Game/RPG/Blueprints/QuestsSystem/QuestsDatas/PDA_Quest.QuestDatas` QuestDatas)))
  (bind (_objectivedatas_id _objectivedatas_name _objectivedatas_description _objectivedatas_type _objectivedatas_approximatelocation _objectivedatas_optional _objectivedatas_optionalexperiencereward _objectivedatas_optionalmoneyreward _objectivedatas_optionalitemsreward _objectivedatas_endstagechecker) (break `/Game/RPG/Blueprints/QuestsSystem/QuestsDatas/S_Objective` (`/Game/RPG/Blueprints/QuestsSystem/QuestsDatas/PDA_Objective.ObjectiveDatas` ObjectiveDatas)))
  (`self.Set Objective Completion` ObjectiveDatas _questdatas_id)
  (if _objectivedatas_endstagechecker
    (bind _allobjectivescompleted (`self.CheckStageFinished` QuestDatas))
    (if _allobjectivescompleted
      (`self.FinishStage` QuestDatas)
      (else
        (bind _quest (`self.GetManipulatedQuestByQuestID` _questdatas_id))
        (bind _result (`self.IsOnlyNotCompletedEndStageChecker` (`|GetArrayItem` _questdatas_stages (`.CurrentStage_10_E1FC846D4FAE690A0C9C04AF3D12109D` (break `/Game/RPG/Blueprints/QuestsSystem/QuestsDatas/S_ManipulatedQuest` _quest))) ObjectiveDatas _questdatas_id))
        (if _result
          (`self.Set Objective Completion` ObjectiveDatas _questdatas_id false))))))

(fn `CreateManipulatedQuest`
  (params (QuestDatas :type "/Game/RPG/Blueprints/QuestsSystem/QuestsDatas/PDA_Quest Object Reference"))
  (returns (ManipulatedQuest :type "/Game/RPG/Blueprints/QuestsSystem/QuestsDatas/S_ManipulatedQuest Structure"))
  (locals (QuestStructure :type "/Game/RPG/Blueprints/QuestsSystem/QuestsDatas/S_ManipulatedQuest Structure") (CurrentStageID :type Integer) (CurrentStageIndex :type Integer :default 0))
  (bind (_queststructure_id _queststructure_stages) (break `/Game/RPG/Blueprints/QuestsSystem/QuestsDatas/S_ManipulatedQuest` (`local.QuestStructure`)))
  (bind (_questdatas_id _questdatas_name _questdatas_description _questdatas_stages) (break `/Game/RPG/Blueprints/QuestsSystem/QuestsDatas/S_Quest` (`/Game/RPG/Blueprints/QuestsSystem/QuestsDatas/PDA_Quest.QuestDatas` QuestDatas)))
  (bind (_queststructure_id_2 _queststructure_stages_2) (break `/Game/RPG/Blueprints/QuestsSystem/QuestsDatas/S_ManipulatedQuest` (`local.QuestStructure`)))
  (bind (_output_id _output_objectives) (break `/Game/RPG/Blueprints/QuestsSystem/QuestsDatas/S_ManipulatedStage` (`|GetArrayItem` _queststructure_stages (`local.CurrentStageIndex`))))
  (set `local.QuestStructure` (make `/Game/RPG/Blueprints/QuestsSystem/QuestsDatas/S_ManipulatedQuest` _questdatas_id))
  (for _array_element _questdatas_stages
    (bind (_stagedatas_id _stagedatas_name _stagedatas_description _stagedatas_objectives) (break `/Game/RPG/Blueprints/QuestsSystem/QuestsDatas/S_Stage` (`/Game/RPG/Blueprints/QuestsSystem/QuestsDatas/PDA_Stage.StageDatas` _array_element)))
    (bind _output_get (set `local.CurrentStageID` _stagedatas_id))
    (bind _returnvalue (`KismetArrayLibrary.Array_AddUnique` _queststructure_stages_2 (make `/Game/RPG/Blueprints/QuestsSystem/QuestsDatas/S_ManipulatedStage` _output_get)))
    (set `local.CurrentStageIndex` _returnvalue)
    (for _array_element_2 _stagedatas_objectives
      (bind _objectivedatas_id (break `/Game/RPG/Blueprints/QuestsSystem/QuestsDatas/S_Objective` (`/Game/RPG/Blueprints/QuestsSystem/QuestsDatas/PDA_Objective.ObjectiveDatas` _array_element_2)))
      (`KismetArrayLibrary.Array_AddUnique` _output_objectives (make `/Game/RPG/Blueprints/QuestsSystem/QuestsDatas/S_ManipulatedObjective` _objectivedatas_id))
      (return (`local.QuestStructure`)))))

(fn `FinishQuest`
  (params (QuestDatas :type "/Game/RPG/Blueprints/QuestsSystem/QuestsDatas/PDA_Quest Object Reference"))
  (bind _questdatas_id (break `/Game/RPG/Blueprints/QuestsSystem/QuestsDatas/S_Quest` (`/Game/RPG/Blueprints/QuestsSystem/QuestsDatas/PDA_Quest.QuestDatas` QuestDatas)))
  (bind _returnvalue (`KismetArrayLibrary.Array_RemoveItem` (`self.StartedQuests`) QuestDatas))
  (if _returnvalue
    (`KismetArrayLibrary.Array_AddUnique` (`self.FinishedQuests`) QuestDatas)
    (`self.GetManipulatedQuestIndexByQuestID` _questdatas_id)
    (`self.SetQuestFinished` _questdatas_id)
    (if (== (`self.ActiveQuest`) QuestDatas)
      (set `self.ActiveQuest` null))))

(fn `FinishStage`
  (params (QuestDatas :type "/Game/RPG/Blueprints/QuestsSystem/QuestsDatas/PDA_Quest Object Reference"))
  (bind (_questdatas_id _questdatas_name _questdatas_description _questdatas_stages) (break `/Game/RPG/Blueprints/QuestsSystem/QuestsDatas/S_Quest` (`/Game/RPG/Blueprints/QuestsSystem/QuestsDatas/PDA_Quest.QuestDatas` QuestDatas)))
  (bind _quest (`self.GetManipulatedQuestByQuestID` _questdatas_id))
  (bind (_stagedatas_id _stagedatas_name _stagedatas_description _stagedatas_objectives) (break `/Game/RPG/Blueprints/QuestsSystem/QuestsDatas/S_Stage` (`/Game/RPG/Blueprints/QuestsSystem/QuestsDatas/PDA_Stage.StageDatas` (`|GetArrayItem` _questdatas_stages (`.CurrentStage_10_E1FC846D4FAE690A0C9C04AF3D12109D` (break `/Game/RPG/Blueprints/QuestsSystem/QuestsDatas/S_ManipulatedQuest` _quest))))))
  (`self.RemoveConsumedItems` _stagedatas_objectives)
  (if (not (> (- (`KismetArrayLibrary.Array_Length` _questdatas_stages) 1) (`.CurrentStage_10_E1FC846D4FAE690A0C9C04AF3D12109D` (break `/Game/RPG/Blueprints/QuestsSystem/QuestsDatas/S_ManipulatedQuest` _quest))))
    (`self.FinishQuest` QuestDatas))
  (`self.SetCurrentStage` QuestDatas (+ (`.CurrentStage_10_E1FC846D4FAE690A0C9C04AF3D12109D` (break `/Game/RPG/Blueprints/QuestsSystem/QuestsDatas/S_ManipulatedQuest` _quest)) 1))
  (`self.ClaimQuestRawards` _questdatas_stages (`.CurrentStage_10_E1FC846D4FAE690A0C9C04AF3D12109D` (break `/Game/RPG/Blueprints/QuestsSystem/QuestsDatas/S_ManipulatedQuest` _quest)) _questdatas_id))

(fn `GetManipulatedObjectiveByUpIDs`
  (params (QuestID :type Integer) (StageID :type Integer) (ObjectiveID :type Integer))
  (returns (Objective :type "/Game/RPG/Blueprints/QuestsSystem/QuestsDatas/S_ManipulatedObjective Structure") (Index :type Integer))
  (bind _index (`self.GetManipulatedQuestIndexByQuestID` QuestID))
  (bind (_output_id _output_stages) (break `/Game/RPG/Blueprints/QuestsSystem/QuestsDatas/S_ManipulatedQuest` (`|GetArrayItem` (`self.ManipulatedQuests`) _index)))
  (bind _index_2 (`self.GetManipulatedStageIndexByStageID` _output_stages StageID))
  (bind (_output_id_2 _output_objectives) (break `/Game/RPG/Blueprints/QuestsSystem/QuestsDatas/S_ManipulatedStage` (`|GetArrayItem` _output_stages _index_2)))
  (bind _index_3 (`self.GetManipulatedObjectiveIndexByObjectiveID` _output_objectives ObjectiveID))
  (return (`|GetArrayItem` _output_objectives _index_3) _index_3))

(fn `GetManipulatedObjectiveIndexByObjectiveID`
  (params (StageObjectives :type "Array of /Game/RPG/Blueprints/QuestsSystem/QuestsDatas/S_ManipulatedObjective Structure") (ObjectiveID :type Integer))
  (returns (Index :type Integer))
  (for (_array_element _array_index) StageObjectives
    (if (== (break `/Game/RPG/Blueprints/QuestsSystem/QuestsDatas/S_ManipulatedObjective` _array_element) ObjectiveID)
      (return _array_index))))

(fn `GetManipulatedQuestByQuestID`
  (params (QuestID :type Integer))
  (returns (Quest :type "/Game/RPG/Blueprints/QuestsSystem/QuestsDatas/S_ManipulatedQuest Structure") (Index :type Integer))
  (for (_array_element _array_index) (`self.ManipulatedQuests`)
    (if (== (break `/Game/RPG/Blueprints/QuestsSystem/QuestsDatas/S_ManipulatedQuest` _array_element) QuestID)
      (return (`|GetArrayItem` (`self.ManipulatedQuests`) _array_index) _array_index))))

(fn `GetManipulatedQuestIndexByQuestID`
  (params (QuestID :type Integer))
  (returns (Index :type Integer))
  (for (_array_element _array_index) (`self.ManipulatedQuests`)
    (if (== (break `/Game/RPG/Blueprints/QuestsSystem/QuestsDatas/S_ManipulatedQuest` _array_element) QuestID)
      (return _array_index))))

(fn `GetManipulatedStageByUpIDs`
  (params (QuestID :type Integer) (StageID :type Integer))
  (returns (Stage :type "/Game/RPG/Blueprints/QuestsSystem/QuestsDatas/S_ManipulatedStage Structure") (Index :type Integer))
  (bind _index (`self.GetManipulatedQuestIndexByQuestID` QuestID))
  (bind (_output_id _output_stages) (break `/Game/RPG/Blueprints/QuestsSystem/QuestsDatas/S_ManipulatedQuest` (`|GetArrayItem` (`self.ManipulatedQuests`) _index)))
  (bind _index_2 (`self.GetManipulatedStageIndexByStageID` _output_stages StageID))
  (return (`|GetArrayItem` _output_stages _index_2) _index_2))

(fn `GetManipulatedStageIndexByStageID`
  (params (QuestStages :type "Array of /Game/RPG/Blueprints/QuestsSystem/QuestsDatas/S_ManipulatedStage Structure") (StageID :type Integer))
  (returns (Index :type Integer))
  (for (_array_element _array_index) QuestStages
    (if (== (break `/Game/RPG/Blueprints/QuestsSystem/QuestsDatas/S_ManipulatedStage` _array_element) StageID)
      (return _array_index))))

(fn `IsOnlyNotCompletedEndStageChecker`
  (params (Stage :type "/Game/RPG/Blueprints/QuestsSystem/QuestsDatas/PDA_Stage Object Reference") (Objective :type "/Game/RPG/Blueprints/QuestsSystem/QuestsDatas/PDA_Objective Object Reference") (QuestID :type Integer))
  (returns (Result :type Boolean))
  (locals (IsTheOnlyOne :type Boolean))
  (bind (_stagedatas_id _stagedatas_name _stagedatas_description _stagedatas_objectives) (break `/Game/RPG/Blueprints/QuestsSystem/QuestsDatas/S_Stage` (`/Game/RPG/Blueprints/QuestsSystem/QuestsDatas/PDA_Stage.StageDatas` Stage)))
  (bind _stagedatas_id_2 (break `/Game/RPG/Blueprints/QuestsSystem/QuestsDatas/S_Stage` (`/Game/RPG/Blueprints/QuestsSystem/QuestsDatas/PDA_Stage.StageDatas` Stage)))
  (set `local.IsTheOnlyOne` true)
  (for (_array_element _array_index) _stagedatas_objectives
    (bind (_objectivedatas_id _objectivedatas_name _objectivedatas_description _objectivedatas_type _objectivedatas_approximatelocation _objectivedatas_optional _objectivedatas_optionalexperiencereward _objectivedatas_optionalmoneyreward _objectivedatas_optionalitemsreward _objectivedatas_endstagechecker) (break `/Game/RPG/Blueprints/QuestsSystem/QuestsDatas/S_Objective` (`/Game/RPG/Blueprints/QuestsSystem/QuestsDatas/PDA_Objective.ObjectiveDatas` _array_element)))
    (bind _objective (`self.GetManipulatedObjectiveByUpIDs` _array_index _stagedatas_id_2 _objectivedatas_id))
    (if (and (!= _array_element Objective) (not (`.IsCompleted_4_0007CAF040ABB7D21F1D118472BE4227` (break `/Game/RPG/Blueprints/QuestsSystem/QuestsDatas/S_ManipulatedObjective` _objective))) (not _objectivedatas_optional) _objectivedatas_endstagechecker)
      (set `local.IsTheOnlyOne` false)
      (break)))
  (return (`local.IsTheOnlyOne`)))

(fn `RemoveConsumedItems`
  (params (Objectives :type "Array of /Game/RPG/Blueprints/QuestsSystem/QuestsDatas/PDA_Objective Object Reference"))
  (for _array_element Objectives
    (bind _aspda_objective_collect (cast `/Game/RPG/Blueprints/QuestsSystem/QuestsDatas/PDA_ObjectiveCollect` _array_element))
    (if (and (`/Game/RPG/Blueprints/QuestsSystem/QuestsDatas/PDA_ObjectiveCollect.Consume` _aspda_objective_collect) false)
      (for _array_element_2 (`/Game/RPG/Blueprints/QuestsSystem/QuestsDatas/PDA_ObjectiveCollect.Items` _aspda_objective_collect)
        (`/Game/RPG/Player/Components/BPC_Inventory.RemoveItem` (`/Game/RPG/Player/BP_Player.PBC_Inventory` (`self.BP Player`)) (break `/Game/RPG/Blueprints/Item/S_ItemSlot` _array_element_2) (`.Amount_7_E08AD9B3421E831788A24AA7FF7CCAA7` (break `/Game/RPG/Blueprints/Item/S_ItemSlot` _array_element_2)))))))

(fn `Set Objective Completion`
  (params (ObjectiveDatas :type "/Game/RPG/Blueprints/QuestsSystem/QuestsDatas/PDA_Objective Object Reference") (QuestID :type Integer) (IsComplete :type Boolean :default true))
  (bind _objectivedatas_id (break `/Game/RPG/Blueprints/QuestsSystem/QuestsDatas/S_Objective` (`/Game/RPG/Blueprints/QuestsSystem/QuestsDatas/PDA_Objective.ObjectiveDatas` ObjectiveDatas)))
  (bind _quest (`self.GetManipulatedQuestByQuestID` QuestID))
  (bind (_output_id _output_objectives) (break `/Game/RPG/Blueprints/QuestsSystem/QuestsDatas/S_ManipulatedStage` (`|GetArrayItem` (`.Stages_12_59DF7918458BD96E23CA02A4A01EEF48` (break `/Game/RPG/Blueprints/QuestsSystem/QuestsDatas/S_ManipulatedQuest` _quest)) (`.CurrentStage_10_E1FC846D4FAE690A0C9C04AF3D12109D` (break `/Game/RPG/Blueprints/QuestsSystem/QuestsDatas/S_ManipulatedQuest` _quest)))))
  (bind (_objective _index) (`self.GetManipulatedObjectiveByUpIDs` (break `/Game/RPG/Blueprints/QuestsSystem/QuestsDatas/S_ManipulatedQuest` _quest) _output_id _objectivedatas_id))
  (`KismetArrayLibrary.Array_Set` _output_objectives _index (make `/Game/RPG/Blueprints/QuestsSystem/QuestsDatas/S_ManipulatedObjective` (break `/Game/RPG/Blueprints/QuestsSystem/QuestsDatas/S_ManipulatedObjective` _objective) IsComplete)))

(fn `SetCurrentStage`
  (params (QuestDatas :type "/Game/RPG/Blueprints/QuestsSystem/QuestsDatas/PDA_Quest Object Reference") (CurrentStage :type Integer))
  (bind _questdatas_id (break `/Game/RPG/Blueprints/QuestsSystem/QuestsDatas/S_Quest` (`/Game/RPG/Blueprints/QuestsSystem/QuestsDatas/PDA_Quest.QuestDatas` QuestDatas)))
  (bind (_quest _index) (`self.GetManipulatedQuestByQuestID` _questdatas_id))
  (`KismetArrayLibrary.Array_Set` (`self.ManipulatedQuests`) _index (make `/Game/RPG/Blueprints/QuestsSystem/QuestsDatas/S_ManipulatedQuest` (break `/Game/RPG/Blueprints/QuestsSystem/QuestsDatas/S_ManipulatedQuest` _quest) (`.Stages_12_59DF7918458BD96E23CA02A4A01EEF48` (break `/Game/RPG/Blueprints/QuestsSystem/QuestsDatas/S_ManipulatedQuest` _quest)) CurrentStage (`.Complete_9_15184102492B1D9CB2602CBD167842BB` (break `/Game/RPG/Blueprints/QuestsSystem/QuestsDatas/S_ManipulatedQuest` _quest)))))

(fn `SetQuestActive`
  (params (QuestDatas :type "/Game/RPG/Blueprints/QuestsSystem/QuestsDatas/PDA_Quest Object Reference"))
  (if (`KismetArrayLibrary.Array_Contains` (`self.StartedQuests`) QuestDatas)
    (set `self.ActiveQuest` QuestDatas)))

(fn `SetQuestFinished`
  (params (QuestID :type Integer))
  (bind (_quest _index) (`self.GetManipulatedQuestByQuestID` QuestID))
  (`KismetArrayLibrary.Array_Set` (`self.ManipulatedQuests`) _index (make `/Game/RPG/Blueprints/QuestsSystem/QuestsDatas/S_ManipulatedQuest` (break `/Game/RPG/Blueprints/QuestsSystem/QuestsDatas/S_ManipulatedQuest` _quest) (`.Stages_12_59DF7918458BD96E23CA02A4A01EEF48` (break `/Game/RPG/Blueprints/QuestsSystem/QuestsDatas/S_ManipulatedQuest` _quest)) (`.CurrentStage_10_E1FC846D4FAE690A0C9C04AF3D12109D` (break `/Game/RPG/Blueprints/QuestsSystem/QuestsDatas/S_ManipulatedQuest` _quest)) true)))

(fn `SetStageRewardsClaimed`
  (params (StageDatas :type "/Game/RPG/Blueprints/QuestsSystem/QuestsDatas/PDA_Stage Object Reference") (QuestID :type Integer))
  (bind _stagedatas_id (break `/Game/RPG/Blueprints/QuestsSystem/QuestsDatas/S_Stage` (`/Game/RPG/Blueprints/QuestsSystem/QuestsDatas/PDA_Stage.StageDatas` StageDatas)))
  (bind _quest (`self.GetManipulatedQuestByQuestID` QuestID))
  (bind (_stage _index) (`self.GetManipulatedStageByUpIDs` (break `/Game/RPG/Blueprints/QuestsSystem/QuestsDatas/S_ManipulatedQuest` _quest) _stagedatas_id))
  (`KismetArrayLibrary.Array_Set` (`.Stages_12_59DF7918458BD96E23CA02A4A01EEF48` (break `/Game/RPG/Blueprints/QuestsSystem/QuestsDatas/S_ManipulatedQuest` _quest)) _index (make `/Game/RPG/Blueprints/QuestsSystem/QuestsDatas/S_ManipulatedStage` (break `/Game/RPG/Blueprints/QuestsSystem/QuestsDatas/S_ManipulatedStage` _stage) (`.Objectives_11_38A887774456D71E5C1987A437AE7B33` (break `/Game/RPG/Blueprints/QuestsSystem/QuestsDatas/S_ManipulatedStage` _stage)) true)))

(fn `UserConstructionScript`)