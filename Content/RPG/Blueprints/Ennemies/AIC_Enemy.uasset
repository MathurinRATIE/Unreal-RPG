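; AI controller for RPG enemies that runs BT_Enemy and turns perception updates into blackboard state.
; BeginPlay caches the controlled enemy and player, then seeds the blackboard with the enemy's patrol spline and starting point index.
; Perception updates record "Hearing"-tagged locations, or otherwise set the player reference when sensed and last-seen location when lost, with debug prints.
; The "Player" tag check is disconnected, so the perceived actor is never filtered.
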(event `self.ReceiveBeginPlay`
  (`self.RunBehaviorTree` "/Game/RPG/Blueprints/Ennemies/BT_Enemy.BT_Enemy")
  (bind _asbp_enemy (cast `/Game/RPG/Blueprints/Ennemies/BP_Enemy` (`self.K2_GetPawn`)))
  (bind _output_get (set `self.BP Enemy` _asbp_enemy))
  (`BlackboardComponent.SetValueAsObject` (`self.Blackboard`) (`self.PatrolSplineKey`) (`/Game/RPG/Blueprints/Ennemies/BP_Enemy.PatrolSpline` _output_get))
  (`BlackboardComponent.SetValueAsInt` (`self.Blackboard`) (`self.PreviousPatrolPointIndexKey`) 0)
  (bind _asbp_player (cast `/Game/RPG/Player/BP_Player` (`GameplayStatics.GetPlayerCharacter` 0)))
  (set `self.BP Player` _asbp_player))

(event `self.AIPerception.OnTargetPerceptionUpdated`
  (params (Actor :type "Actor Object Reference") (Stimulus :type "AIStimulus Structure"))
  (bind (_age _expirationage _strength _stimuluslocation _receiverlocation _tag _bsuccessfullysensed) (break `AIStimulus` Stimulus))
  (if (== _tag "Hearing")
    (`KismetSystemLibrary.PrintString` "Heared")
    (`BlackboardComponent.SetValueAsVector` (`self.Blackboard`) (`self.LastHearingLocationKey`) _stimuluslocation)
    (elif _bsuccessfullysensed
      (`KismetSystemLibrary.PrintString` "Seen")
      (`BlackboardComponent.ClearValue` (`self.Blackboard`) (`self.LastSeenLocactionKey`))
      (`BlackboardComponent.SetValueAsObject` (`self.Blackboard`) (`self.PlayerRefKey`) (`self.BP Player`))
      (`BlackboardComponent.ClearValue` (`self.Blackboard`) (`self.LastHearingLocationKey`))
      (else
        (`KismetSystemLibrary.PrintString` "Unseen")
        (`BlackboardComponent.SetValueAsVector` (`self.Blackboard`) (`self.LastSeenLocactionKey`) _stimuluslocation)
        (`BlackboardComponent.ClearValue` (`self.Blackboard`) (`self.PlayerRefKey`))
        (`BlackboardComponent.ClearValue` (`self.Blackboard`) (`self.LastHearingLocationKey`))))))

(fn `UserConstructionScript`)