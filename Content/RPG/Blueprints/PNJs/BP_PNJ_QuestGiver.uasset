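; Quest-giver NPC Blueprint that hands a quest to the player through dialogue.
; It overrides EndDialogue: after the parent logic, the first completed dialogue calls ClaimQuest on the player's QuestsManager and sets QuestGiven.
; Later dialogue endings switch Dialogues to QuestGivenDialogue, so the swap happens one conversation after the quest is claimed.
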(fn `EndDialogue`
  (`parent.EndDialogue`)
  (if (`self.QuestGiven`)
    (set `self.Dialogues` (`self.QuestGivenDialogue`))
    (else
      (`/Game/RPG/Blueprints/QuestsSystem/BP_QuestsManager.ClaimQuest` (`/Game/RPG/Player/BP_Player.QuestsManager` (`/Game/RPG/_Common/PC_Player.BP Player` (`self.PC Player`))) (`self.Quest`))
      (set `self.QuestGiven` true))))

(fn `UserConstructionScript`
  (`parent.UserConstructionScript`))