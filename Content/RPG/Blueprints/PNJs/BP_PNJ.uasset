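; BP_PNJ is an RPG NPC that the player can talk to and that feeds interaction quest objectives.
; An overlap radius shows the interact prompt and registers the NPC on the player controller.
; StartDialogue switches to UI-only input and the dialogue widget, then NextDialogue steps through the Dialogues array.
; Starting and ending check QuestsManager objectives; ending also restores game input and resets the index to FirstDialogueOnRepeat.
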(event `self.ReceiveBeginPlay`
  (set `self.CurrentDialogueIndex` 0)
  (bind _aspc_player (cast `/Game/RPG/_Common/PC_Player` (`GameplayStatics.GetPlayerController` 0)))
  (set `self.PC Player` _aspc_player))

(event `self.IntreractRadius.OnComponentBeginOverlap`
  (params (OverlappedComponent :type "PrimitiveComponent Object Reference") (OtherActor :type "Actor Object Reference") (OtherComp :type "PrimitiveComponent Object Reference") (OtherBodyIndex :type Integer) (bFromSweep :type Boolean) (SweepResult :type "HitResult Structure (by ref)"))
  (if (`self.ActorHasTag` OtherActor "Player")
    (`Widget.SetVisibility` (`/Game/RPG/_Common/PC_Player.WBP_Interact` (`self.PC Player`)) "Visible")
    (set `/Game/RPG/_Common/PC_Player.InteractablePNJ` self (`self.PC Player`))))

(event `self.IntreractRadius.OnComponentEndOverlap`
  (params (OverlappedComponent :type "PrimitiveComponent Object Reference") (OtherActor :type "Actor Object Reference") (OtherComp :type "PrimitiveComponent Object Reference") (OtherBodyIndex :type Integer))
  (if (`self.ActorHasTag` OtherActor "Player")
    (if (== (`/Game/RPG/_Common/PC_Player.InteractablePNJ` (`self.PC Player`)) self)
      (`Widget.SetVisibility` (`/Game/RPG/_Common/PC_Player.WBP_Interact` (`self.PC Player`)) "Hidden")
      (set `/Game/RPG/_Common/PC_Player.InteractablePNJ` null (`self.PC Player`)))))

(fn `CloseDialogueWidget`
  (`Widget.SetVisibility` (`/Game/RPG/_Common/PC_Player.WBP_Interact` (`self.PC Player`)) "Visible")
  (`Widget.SetVisibility` (`/Game/RPG/_Common/PC_Player.WBP_InGame` (`self.PC Player`)) "Visible")
  (`Widget.SetVisibility` (`/Game/RPG/_Common/PC_Player.WBP_Dialogue` (`self.PC Player`)) "Hidden")
  (set `PlayerController.bShowMouseCursor` false (`self.PC Player`))
  (`WidgetBlueprintLibrary.SetInputMode_GameOnly` (`self.PC Player`))
  (`Widget.SetVisibility` (`/Game/RPG/_Common/PC_Player.WBP_Dialogue` (`self.PC Player`)) "Hidden"))

(fn `DisplayCurrentDialogue`
  (set `TextBlock.Text` (`|GetArrayItem` (`self.Dialogues`) (`self.CurrentDialogueIndex`)) (`/Game/RPG/UI/Dialogue/WBP_Dialogue.Dialogue` (`/Game/RPG/_Common/PC_Player.WBP_Dialogue` (`self.PC Player`)))))

(fn `EndDialogue`
  (set `self.CurrentDialogueIndex` (`self.FirstDialogueOnRepeat`))
  (`self.CloseDialogueWidget`)
  (set `self.DialogueStarted` false)
  (`/Game/RPG/Blueprints/QuestsSystem/QuestsManager.CheckInteractObjectives` (`/Game/RPG/Player/BP_Player.QuestsManager` (`/Game/RPG/_Common/PC_Player.BP Player` (`self.PC Player`))) null))

(fn `NextDialogue`
  (bind _currentdialogueindex (`self.CurrentDialogueIndex`))
  (if (`self.DialogueStarted`)
    (`/Engine/EditorBlueprintResources/StandardMacros.IncrementInt` _currentdialogueindex
      (:`  `
        (if (< _currentdialogueindex (`KismetArrayLibrary.Array_Length` (`self.Dialogues`)))
          (`self.DisplayCurrentDialogue`)
          (else
            (`self.EndDialogue`)))))))

(fn `OpenDialogueWidget`
  (bind (_returnvalue_x _returnvalue_y) (`KismetMathLibrary.BreakVector2D` (`WidgetLayoutLibrary.GetViewportSize`)))
  (`Widget.SetVisibility` (`/Game/RPG/_Common/PC_Player.WBP_Interact` (`self.PC Player`)) "Hidden")
  (`Widget.SetVisibility` (`/Game/RPG/_Common/PC_Player.WBP_InGame` (`self.PC Player`)) "Hidden")
  (`Widget.SetVisibility` (`/Game/RPG/_Common/PC_Player.WBP_Dialogue` (`self.PC Player`)) "Visible")
  (`PlayerController.SetMouseLocation` (`self.PC Player`) (`KismetMathLibrary.FTrunc` (* _returnvalue_x 0.5)) (`KismetMathLibrary.FTrunc` (- _returnvalue_y 450.0)))
  (set `PlayerController.bShowMouseCursor` true (`self.PC Player`))
  (`WidgetBlueprintLibrary.SetFocusToGameViewport`)
  (`WidgetBlueprintLibrary.SetInputMode_UIOnlyEx` (`self.PC Player`) (`/Game/RPG/_Common/PC_Player.WBP_Dialogue` (`self.PC Player`)))
  (set `/Game/RPG/UI/Dialogue/WBP_Dialogue.PNJ` self (`/Game/RPG/_Common/PC_Player.WBP_Dialogue` (`self.PC Player`))))

(fn `StartDialogue`
  (locals (WBP_Dialogue :type "/Game/RPG/UI/Dialogue/WBP_Dialogue Object Reference"))
  (set `self.DialogueStarted` true)
  (`self.OpenDialogueWidget`)
  (set `TextBlock.Text` (`KismetTextLibrary.Conv_StringToText` (`self.Name`)) (`/Game/RPG/UI/Dialogue/WBP_Dialogue.Name` (`/Game/RPG/_Common/PC_Player.WBP_Dialogue` (`self.PC Player`))))
  (`self.DisplayCurrentDialogue`)
  (`/Game/RPG/Blueprints/QuestsSystem/QuestsManager.CheckInteractObjectives` (`/Game/RPG/Player/BP_Player.QuestsManager` (`/Game/RPG/_Common/PC_Player.BP Player` (`self.PC Player`))) self))

(fn `UserConstructionScript`)