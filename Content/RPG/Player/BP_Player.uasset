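; BP_Player is the RPG player Blueprint, holding health, armor, stamina, money, experience and level.
; On BeginPlay it caches PC_Player and the quest manager, then initializes stats and the in-game HUD.
; Stat functions push changes straight to that widget, while AddExp loops through level-ups against an exponentially growing threshold.
; A debug key emits a "Hearing" noise at the player's location.
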(event EventBeginPlay
  (bind _aspc_player (Utilities|Casting|CastToPC_Player (Game|GetPlayerController 0)))
  (Variables|Default|SetPC%20Player _aspc_player)
  (CallFunction|UpdateHealth (Variables|Stats|Max|GetMaxHealth))
  (CallFunction|UpdateArmorPoints (Variables|Stats|GetArmorPoints))
  (CallFunction|UpdateStamina (Variables|Stats|Max|GetMaxStamina))
  (bind _returnvalue (Actor|GetActorOfClass "/Game/RPG/Blueprints/QuestsSystem/BP_QuestsManager.BP_QuestsManager_C"))
  (Variables|Default|SetQuestsManager _returnvalue)
  (Default|UpdateMoney (Variables|/Game/RPG/_Common/PC_Player.PC_Player_C|GetWBP_InGame (Variables|Default|GetPC%20Player)) (Variables|Stats|GetMoney))
  (CallFunction|CalculateCurrentLevelExp)
  (Default|UpdateExp (Variables|/Game/RPG/_Common/PC_Player.PC_Player_C|GetWBP_InGame (Variables|Default|GetPC%20Player)) (Variables|Stats|GetExp) (Variables|Stats|GetCurrentLevelExp))
  (Default|UpdateLevel (Variables|/Game/RPG/_Common/PC_Player.PC_Player_C|GetWBP_InGame (Variables|Default|GetPC%20Player)) (Variables|Stats|GetLevel)))

(event Input|KeyboardEvents|DebugKeyA
  (params (Key :type Key%20Structure) (ActionValue :type Input%20Action%20Value%20Structure))
  (:Pressed
    (Class|Actor|MakeNoise 1.0 0 (Transformation|GetActorLocation) 0.0 "Hearing")))

(fn ConstructionScript)

(fn UpdateHealth
  (params (Health :type Float%20%28double-precision%29))
  (if (<= Health (Variables|Stats|Max|GetMaxHealth))
    (bind _output_get (Variables|Stats|SetCurrentHealth Health))
    (else
      (Variables|Stats|SetCurrentHealth (Variables|Stats|Max|GetMaxHealth))))
  (Default|UpdateHealth (Variables|/Game/RPG/_Common/PC_Player.PC_Player_C|GetWBP_InGame (Variables|Default|GetPC%20Player)) _output_get (Variables|Stats|Max|GetMaxHealth)))

(fn UpdateArmorPoints
  (params (ArmorPoints :type Float%20%28double-precision%29))
  (bind _output_get (Variables|Stats|SetArmorPoints ArmorPoints))
  (Default|UpdateArmorPoints (Variables|/Game/RPG/_Common/PC_Player.PC_Player_C|GetWBP_InGame (Variables|Default|GetPC%20Player)) _output_get))

(fn UpdateStamina
  (params (CurrentStamina :type Float%20%28double-precision%29))
  (Variables|Stats|SetCurrentStamina CurrentStamina)
  (Default|UpdateStamina (Variables|/Game/RPG/_Common/PC_Player.PC_Player_C|GetWBP_InGame (Variables|Default|GetPC%20Player)) (Variables|Stats|GetCurrentStamina) (Variables|Stats|Max|GetMaxStamina)))

(fn AddMoney
  (params (Money :type Float%20%28double-precision%29))
  (bind _output_get (Variables|Stats|SetMoney (+ Money (Variables|Stats|GetMoney))))
  (Default|UpdateMoney (Variables|/Game/RPG/_Common/PC_Player.PC_Player_C|GetWBP_InGame (Variables|Default|GetPC%20Player)) _output_get))

(fn RemoveMoney
  (params (Money :type Float%20%28double-precision%29))
  (bind _output_get (Variables|Stats|SetMoney (- Money (Variables|Stats|GetMoney))))
  (Default|UpdateMoney (Variables|/Game/RPG/_Common/PC_Player.PC_Player_C|GetWBP_InGame (Variables|Default|GetPC%20Player)) _output_get))

(fn AddExp
  (params (Exp :type Float%20%28double-precision%29))
  (bind _output_get (Variables|Stats|SetExp (+ Exp (Variables|Stats|GetExp))))
  (Default|UpdateExp (Variables|/Game/RPG/_Common/PC_Player.PC_Player_C|GetWBP_InGame (Variables|Default|GetPC%20Player)) _output_get 0.0)
  (if (>= _output_get (Variables|Stats|GetCurrentLevelExp)) :!label _label
    (Variables|Stats|SetExp (- (Variables|Stats|GetExp) (Variables|Stats|GetCurrentLevelExp)))
    (bind _result (Math|Integer|IncrementInt (Variables|Stats|GetLevel))
      (:%20%20
        (Default|UpdateLevel (Variables|/Game/RPG/_Common/PC_Player.PC_Player_C|GetWBP_InGame (Variables|Default|GetPC%20Player)) _result)
        (CallFunction|CalculateCurrentLevelExp)
        (Default|UpdateExp (Variables|/Game/RPG/_Common/PC_Player.PC_Player_C|GetWBP_InGame (Variables|Default|GetPC%20Player)) (Variables|Stats|GetExp) (Variables|Stats|GetCurrentLevelExp))
        (goto _label)))))

(fn CalculateCurrentLevelExp
  (Variables|Stats|SetCurrentLevelExp (* (Variables|Stats|Max|GetBaseLevelExp) (Math|Float|Power (Variables|Stats|Max|GetLevelExpMultiplier) (Math|Conversions|ToFloat(Integer) (Variables|Stats|GetLevel))))))